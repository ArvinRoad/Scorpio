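; Deathmatch game mode that registers joining players, spawns their characters and refreshes the scoreboard.
; On PostLogin it starts each BP_FPSPlayerController's spawn flow and stores a name and zero score in a map keyed by controller.
; RequestSpark spawns BP_Attacker at PlayerStarts gathered on BeginPlay, cycling through them round-robin.
; UpdateValues pushes all players' data to every registered controller.
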(event `self.K2_PostLogin`
  (params (NewPlayer :type "PlayerController Object Reference"))
  ;[1 1 1] 当玩家链接进来记录玩家的Player Controller 传入（代表该玩家加入游戏中）
  ;[1 1 1] 以该类型生成玩家
  (bind _asbp_fpsplayer_controller (cast `/Game/_Scorpio/Blueprint/Games/BP_FPSPlayerController` NewPlayer))
  ;[1 1 1] 延迟（生成玩家<BP_FPASPlayerController 定义蓝图方法>）
  (`/Game/_Scorpio/Blueprint/Games/BP_FPSPlayerController.StartSparkCharacter` _asbp_fpsplayer_controller)
  ;[1 1 1] 将加入玩家数据存入 Play Game Data Map （数据信息存放在C++ KismetFPSLibrary ）
  (`BlueprintMapLibrary.Map_Add` (`self.PlayerGameDataMap`) _asbp_fpsplayer_controller (make `DeathMatchPlayerData` (`KismetStringLibrary.Conv_StringToName` (`KismetSystemLibrary.GetObjectName` _asbp_fpsplayer_controller)))))

(event `self.ReceiveBeginPlay`
  ;[1 1 1] 初始化玩家出生坐标信息
  (bind _outactors (`GameplayStatics.GetAllActorsOfClass` "/Script/Engine.PlayerStart"))
  (set `self.CharacterSpawnPoints` _outactors))

(event `RequestSpark`
  (params (PlayerController :type "/Game/_Scorpio/Blueprint/Games/BP_FPSPlayerController Object Reference"))
  ;[1 1 1] Request 玩家信息
  (`/Game/_Scorpio/Blueprint/Games/BP_FPSPlayerController.SpawnPlayerCharacter` PlayerController "/Game/_Scorpio/Blueprint/Players/BP_Attacker.BP_Attacker_C" (`self.GetTransform` (`|GetArrayItem` (`self.CharacterSpawnPoints`) (`self.SpawnIdex`))))
  (set `self.SpawnIdex` (+ (`self.SpawnIdex`) 1))
  (if (>= (`self.SpawnIdex`) (`KismetArrayLibrary.Array_Length` (`self.CharacterSpawnPoints`)))
    ;[1 1 1] 回到第一个位置进行生成
    (set `self.SpawnIdex` 0)))

(event `UpdateValues`
  ;[1 1 1] 刷新更新排行榜
  (bind _keys (`BlueprintMapLibrary.Map_Keys` (`self.PlayerGameDataMap`)))
  (for _array_element _keys
    (bind _values (`BlueprintMapLibrary.Map_Values` (`self.PlayerGameDataMap`)))
    (`/Game/_Scorpio/Blueprint/Games/BP_FPSPlayerController.UpdateValues` _array_element _values)))

(fn `UserConstructionScript`)